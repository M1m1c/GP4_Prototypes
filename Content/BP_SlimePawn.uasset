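; Slime player pawn whose sphere deforms through material parameters driven by six directional deform nodes.
; BeginPlay snaps the camera holder and nodes to the actor's location.
; Each tick, the camera holder eases toward a point above the pawn, and the arrow and sphere orient to the movement component's main force.
; DeformDir then feeds each node's direction and clamped distance from the sphere into its materials.
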(event EventBeginPlay
  (bind _returnvalue (Transformation|GetActorLocation))
  (Transformation|SetWorldLocation (Variables|Default|GetcameraHolder) _returnvalue false false)
  (Transformation|SetWorldLocation (Variables|Default|GetTopDeformNode) _returnvalue false false)
  (Transformation|SetWorldLocation (Variables|Default|GetBottomDeformNode) _returnvalue false false)
  (Transformation|SetWorldLocation (Variables|Default|GetForwardDeformNode) _returnvalue false false)
  (Transformation|SetWorldLocation (Variables|Default|GetBackDeformNode) _returnvalue false false)
  (Transformation|SetWorldLocation (Variables|Default|GetRightDeformNode) _returnvalue false false)
  (Transformation|SetWorldLocation (Variables|Default|GetLeftDeformNode) _returnvalue false false))

(event Collision|EventActorBeginOverlap
  (params (OtherActor :type Actor%20Object%20Reference)))

(event EventTick
  (params (DeltaSeconds :type Float%20%28single-precision%29))
  (bind _cameraholder (Variables|Default|GetcameraHolder))
  (Transformation|SetWorldLocation _cameraholder (Math|Vector|Lerp(Vector) (Transformation|GetWorldLocation _cameraholder) (+ (Transformation|GetActorLocation) "0,0,50.000000") (* DeltaSeconds 5.0)) false false)
  (bind _returnvalue (Class|MovementComp|GetMainForce (Variables|Default|GetmovementComp)))
  (Transformation|SetWorldRotation (Variables|Default|GetArrow) (Math|Conversions|ToRotator(Quat) (Math|Vector4|MakeVector4 (.X (Math|Vector|BreakVector _returnvalue)) (.Y (Math|Vector|BreakVector _returnvalue)) (.Z (Math|Vector|BreakVector _returnvalue)) 0.0)) false false)
  (Transformation|SetWorldRotation (Variables|Default|GetSphere) (Math|Conversions|ToRotator(Quat) (Math|Vector4|MakeVector4 (.X (Math|Vector|BreakVector _returnvalue)) (.Y (Math|Vector|BreakVector _returnvalue)) (.Z (Math|Vector|BreakVector _returnvalue)) 0.0)) false false)
  (CallFunction|DeformDir "TopDirection" (Variables|Default|GetTopDeformNode) "TopMagnitude")
  (CallFunction|DeformDir "BottomDirection" (Variables|Default|GetBottomDeformNode) "BottomMagnitude")
  (CallFunction|DeformDir "FrontDirection" (Variables|Default|GetForwardDeformNode) "FrontMagnitude")
  (CallFunction|DeformDir "BackDirection" (Variables|Default|GetBackDeformNode) "BackMagnitude")
  (CallFunction|DeformDir "RightDirection" (Variables|Default|GetRightDeformNode) "RightMagnitude")
  (CallFunction|DeformDir "LeftDirection" (Variables|Default|GetLeftDeformNode) "LeftMagnitude"))

(fn ConstructionScript)

(fn DeformDir
  (params (VectorName :type Name) (DeformMatTarget :type Scene%20Component%20Object%20Reference) (ScalarName :type Name))
  (bind _returnvalue (Transformation|GetWorldLocation DeformMatTarget))
  (bind _sphere (Variables|Default|GetSphere))
  (bind _returnvalue_2 (Transformation|GetWorldLocation _sphere))
  (Rendering|Material|SetVectorParameterValueonMaterials _sphere VectorName (Math|Vector|GetUnitDirection(Vector) _returnvalue_2 _returnvalue))
  (Rendering|Material|SetScalarParameterValueonMaterials _sphere ScalarName (Math|Float|Max(Float) (Math|Vector|Distance(Vector) _returnvalue_2 _returnvalue) 0.1)))